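; BaseEnemyUnit_BP is the base Blueprint for enemy units in battle, extending a parent unit class.
; On BeginPlay it sets the cursor widget's image to the enemy cursor.
; When its turn becomes active, it runs the parent logic, then sets the IsTurn Blackboard key to true on its AI controller.
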(event EventBeginPlay
  (|CallParentFunction)
  (Variables|/Game/Blueprints/UI/CursorUI_BP.CursorUI_BP_C|SetCursorImage (Variables|Default|GetCursorWidget) "/Game/Blueprints/UI/Textures/Battle/Enemy_Cursor.Enemy_Cursor"))

(event Collision|EventActorBeginOverlap
  (params (OtherActor :type Actor%20Object%20Reference))
  (|CallParentFunction OtherActor) ; This node is disabled and will not be called.\nDrag off pins to build functionality.
)

(event EventTick
  (params (DeltaSeconds :type Float%20%28single-precision%29))
  (|CallParentFunction DeltaSeconds) ; This node is disabled and will not be called.\nDrag off pins to build functionality.
)

(event EventSetActiveTurn
  ;[0 0 0] Sets BB Key Is Turn to TRUE
  (|CallParentFunction)
  (AI|Components|Blackboard|SetValueasBool (Variables|/Script/AIModule.AIController|GetBlackboard (AI|GetAIController self)) (Variables|Default|GetIsTurn) true))

(fn ConstructionScript
  (|CallParentFunction))