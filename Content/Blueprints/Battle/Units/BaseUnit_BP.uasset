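; Base battle unit for an FFX-style game, handling movement to a target and back, a miss animation, and death.
; BeginPlay caches the game mode, cursor widget and starting transform.
; MoveToTarget hides the current-character icon, faces the target and lerps there by timeline, then fires OnMovedToTarget.
; MoveToStart uses another timeline to return and restore rotation; Dead destroys the actor after a delay, and SetActiveTurn is empty.
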(event Custom|Dead
  ;[0 0 0] Destroys Actor when DEAD
  (Utilities|FlowControl|Delay 1.0)
  (Actor|DestroyActor))

(event Custom|MoveToStart
  (bind _self self)
  (bind _self_2 self)
  (bind _startlocation (Variables|Default|GetStartLocation))
  (bind _returnvalue (Transformation|GetActorLocation _self))
  ;[0 0 0] Rotates and Moves Character back to Start Position
  (Transformation|SetActorRotation _self (Math|Rotator|FindLookatRotation _returnvalue _startlocation))
  (bind _alpha (Timeline|MoveToStartTimeline PlayFromStart)
    (:Update
      (Transformation|SetActorLocation _self_2 (Math|Vector|Lerp(Vector) _startlocation _returnvalue _alpha) false false))
    (:Finished
      (Transformation|SetActorRotation _self_2 (Variables|Default|GetStartRotation)))))

(event Custom|MoveToTarget
  (params (TargetLocation :type Vector))
  ;[0 0 0] Hides Purple Triangle Icon
  (Rendering|SetVisibility (Variables|Default|GetCurrentCharacterIcon) false false)
  ;[0 0 0] Character Faces Target
  (Transformation|SetActorRotation self (Math|Rotator|FindLookatRotation (Variables|Default|GetStartLocation) TargetLocation))
  ;[0 0 0] Character moves to Target & Calls Event Dispatcher on Completion
  (bind _alpha (Timeline|MoveToTargetTimeline PlayFromStart)
    (:Update
      (Transformation|SetActorLocation self (Math|Vector|Lerp(Vector) (Variables|Default|GetStartLocation) TargetLocation _alpha) false false))
    (:Finished
      (Default|CallOnMovedtoTarget))))

(event Custom|PlayMissAnimation
  (Animation|PlayAnimMontage (Variables|Default|GetMissAnimation) 1.0 "None"))

(event Custom|SetActiveTurn)

(event EventBeginPlay
  (bind _self self)
  (bind _asffxgame_mode_bp (Utilities|Casting|CastToFFXGameMode_BP (Game|GetGameMode)))
  (Variables|Default|SetGameMode _asffxgame_mode_bp)
  (bind _ascursor_ui_bp (Utilities|Casting|CastToCursorUI_BP (UserInterface|GetWidget (Variables|Default|GetCursor%20UI))))
  (Variables|Default|SetCursorWidget _ascursor_ui_bp)
  (Variables|Default|SetStartLocation (Transformation|GetActorLocation _self))
  (Variables|Default|SetStartRotation (Transformation|GetActorRotation _self)))

(event Collision|EventActorBeginOverlap
  (params (OtherActor :type Actor%20Object%20Reference)))

(event EventTick
  (params (DeltaSeconds :type Float%20%28single-precision%29)))

(fn ConstructionScript)