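; Base battle Blueprint for an FFX-style game that spawns combatants at fixed spawn components and hands off to BattleController.
; InitBattle disables player input, spawns the party from GameMode stats with DataTable-driven equipment meshes, and spawns enemies from BattleCharacters_DT.
; Placeholder ranges currently limit this to one Tidus and one fixed enemy row; inactive-party spawning is uncalled.
; Separate events destroy combatants and save collected gil and items to the GameMode.
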(event Custom|InitBattle
  ;[0 0 0] Initialize's Battle & Battle Controller
  (Default|DisablePlayerInput (Variables|Overall|GetFFXGameMode))
  (CallFunction|SpawnActiveParty)
  (CallFunction|SpawnEnemies)
  (Utilities|Map|Clear (Variables|BattleEnd|GetCollected%20Items))
  (Variables|BattleEnd|SetCollected%20Gil 0)
  (Default|InitBattle (Variables|Overall|GetBattleController) self (Variables|Overall|GetFFXGameMode)))

(event Custom|Spawn%20Active%20Party
  ;[0 0 0] Spawns Active Party - CHANGE INDICES WHEN APPLICABLE
  (for _index (range 0 0)
    (switch name (Utilities|Array|Get(acopy) (Variables|/Game/Blueprints/FFXGameMode_BP.FFXGameMode_BP_C|GetParty (Variables|Overall|GetFFXGameMode)) _index)
      (:Tidus
        (Variables|Overall|SetSpawnClass "/Game/Blueprints/Battle/Units/Players/Tidus_Battle_BP.Tidus_Battle_BP_C")
        (Variables|Overall|SetCharacterStats (Variables|/Game/Blueprints/FFXGameMode_BP.FFXGameMode_BP_C|GetTidusStats (Variables|Overall|GetFFXGameMode)))
        (bind _returnvalue (Game|SpawnActorfromClass (Variables|Overall|GetSpawnClass) (Math|Transform|MakeTransform (Transformation|GetWorldLocation (Utilities|Array|Get(acopy) (Variables|ActiveParty|GetActivePartySpawnLocations) _index)) (Transformation|GetWorldRotation (Utilities|Array|Get(acopy) (Variables|ActiveParty|GetActivePartySpawnLocations) _index))) "Undefined" "MultiplyWithRoot" 0 0))
        (bind _output_get (Variables|/Game/Blueprints/Battle/Units/BaseUnit_BP.BaseUnit_BP_C|SetCharacterStats_BPC _returnvalue (Variables|Overall|GetCharacterStats)))
        (Utilities|SetCharacterEquipment _output_get (Utilities|Array|Get(acopy) (Variables|/Game/Blueprints/FFXGameMode_BP.FFXGameMode_BP_C|GetParty (Variables|Overall|GetFFXGameMode)) _index) _returnvalue
          (:Out
            (Utilities|Array|Add (Variables|ActiveParty|GetActivePlayerCharacters) _returnvalue)))))))

(event Custom|Spawn%20Enemies
  ;[0 0 0] Gets random enemies from DT and spawns them
  (bind _rownames (Utilities|GetRandomEnemyList)
    (:Out
      (for (_array_element _array_index) _rownames
        (bind _returnvalue (Utilities|GetDataTableRow "/Game/Blueprints/DataTables/Battle_Specfic/BattleCharacters_DT.BattleCharacters_DT" _array_element)
          (:then
            (bind _returnvalue_2 (Game|SpawnActorfromClass (.enemybp _returnvalue) (Math|Transform|MakeTransform (Transformation|GetWorldLocation (Utilities|Array|Get(acopy) (Variables|EnemyParty|GetEnemySpawnLocations) _array_index)) (Transformation|GetWorldRotation (Utilities|Array|Get(acopy) (Variables|EnemyParty|GetEnemySpawnLocations) _array_index))) "Undefined" "MultiplyWithRoot" 0 0))
            (Default|SetCurrentBattle _returnvalue_2 self)
            (Utilities|Array|Add (Variables|EnemyParty|GetEnemyCharacters) _returnvalue_2)))))))

(event Custom|Spawn%20Inactive%20Party
  ;[0 0 0] Inactive Party Spawn - CHANGE INDICES WHEN APPLICABLE & NOT ON AT THE MOMENT
  (for _index (range 0 0)
    (switch name (Utilities|Array|Get(acopy) (Variables|/Game/Blueprints/FFXGameMode_BP.FFXGameMode_BP_C|GetParty (Variables|Overall|GetFFXGameMode)) _index)
      (:Tidus
        (Variables|Overall|SetSpawnClass "/Game/Blueprints/Battle/Units/Players/Tidus_Battle_BP.Tidus_Battle_BP_C")
        (Variables|Overall|SetCharacterStats (Variables|/Game/Blueprints/FFXGameMode_BP.FFXGameMode_BP_C|GetTidusStats (Variables|Overall|GetFFXGameMode)))
        (bind _returnvalue (Game|SpawnActorfromClass (Variables|Overall|GetSpawnClass) (Math|Transform|MakeTransform (Transformation|GetWorldLocation (Utilities|Array|Get(acopy) (Variables|InactiveParty|GetInactivePartySpawnLocations) _index)) (Transformation|GetWorldRotation (Utilities|Array|Get(acopy) (Variables|InactiveParty|GetInactivePartySpawnLocations) _index))) "Undefined" "MultiplyWithRoot" 0 0))
        (Variables|/Game/Blueprints/Battle/Units/BaseUnit_BP.BaseUnit_BP_C|SetCharacterStats_BPC _returnvalue (Variables|Overall|GetCharacterStats))
        (Utilities|Array|Add (Variables|InactiveParty|GetInactivePlayerCharacters) _returnvalue)))))

(event Custom|RemoveUnits
  (bind _enemycharacters (Variables|EnemyParty|GetEnemyCharacters))
  (bind _activeplayercharacters (Variables|ActiveParty|GetActivePlayerCharacters))
  ;[0 0 0] Clears Character Arrays
  (for _array_element _activeplayercharacters
    (Actor|DestroyActor _array_element))
  (Utilities|Array|Clear _activeplayercharacters)
  (for _array_element_2 _enemycharacters
    (Actor|DestroyActor _array_element_2))
  (Utilities|Array|Clear _enemycharacters))

(event Custom|Save%20Collected%20Stuff%20to%20Game%20Mode
  (bind _ffxgamemode (Variables|Overall|GetFFXGameMode))
  ;[0 0 0] Sets Gil
  (Variables|/Game/Blueprints/FFXGameMode_BP.FFXGameMode_BP_C|SetTotalGil _ffxgamemode (+ (Variables|/Game/Blueprints/FFXGameMode_BP.FFXGameMode_BP_C|GetTotalGil _ffxgamemode) (Variables|BattleEnd|GetCollected%20Gil)))
  ;[0 0 0] Adds Use Items
  (Default|AddUseItemstoInventory (Variables|/Game/Blueprints/FFXGameMode_BP.FFXGameMode_BP_C|GetInventory _ffxgamemode) (Variables|BattleEnd|GetCollected%20Items)))

(event EventBeginPlay
  ;[0 0 0] Added Player Spawns Components to Array Variable
  (Variables|ActiveParty|SetActivePartySpawnLocations (Utilities|Array|MakeArray (Variables|Default|GetPlayer%20Spawn%201) (Variables|Default|GetPlayer%20Spawn%202) (Variables|Default|GetPlayer%20Spawn%203)))
  (Variables|InactiveParty|SetInactivePartySpawnLocations (Utilities|Array|MakeArray (Variables|Default|GetInactive%20Spawn%201) (Variables|Default|GetInactive%20Spawn%202) (Variables|Default|GetInactive%20Spawn%203)))
  (Variables|EnemyParty|SetEnemySpawnLocations (Utilities|Array|MakeArray (Variables|Default|GetEnemy%20Spawn%201) (Variables|Default|GetEnemy%20Spawn%202) (Variables|Default|GetEnemy%20Spawn%203)))
  ;[0 0 0] Saving Gamemode as Variable
  (bind _asffxgame_mode_bp (Utilities|Casting|CastToFFXGameMode_BP (Game|GetGameMode))
    (:then
      (Variables|Overall|SetFFXGameMode _asffxgame_mode_bp))
    (:CastFailed
      (Development|PrintString "Game Mode is not FFX Game Mode"))))

(fn ConstructionScript)