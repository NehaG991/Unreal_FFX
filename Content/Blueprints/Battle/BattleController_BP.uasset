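; Battle controller that moves the game between exploration and battle for a given battle instance.
; InitBattle stores the battle and game mode, sets the battle state, blends the view to the battle camera and creates the battle UI.
; A test delay then ends the battle automatically, restoring explore state, player input and the Tidus camera, collapsing the UI and removing units.
; Camera-switch macros validate their targets before changing view.
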(event Custom|InitBattle
  (params (Battle :type Battle%20Base%20BP%20Object%20Reference) (Game%20Mode :type FFX%20Game%20Mode%20BP%20Object%20Reference))
  ;[0 0 0] Gets Initial Battle Info
  (Variables|Default|SetCurrentBattle Battle)
  (Variables|Default|SetFFXGameMode Game%20Mode)
  (CallFunction|SwitchtoBattleMode))

(event Custom|SwitchToBattleMode
  ;[0 0 0] Switches Game State to Battle
  (Variables|/Game/Blueprints/FFXGameMode_BP.FFXGameMode_BP_C|SetCurrentGameState (Variables|Default|GetFFXGameMode) "NewEnumerator1")
  (CallFunction|StartBattle))

(event Custom|StartBattle
  ;[0 0 0] Starts Battle
  (Utilities|SwitchtoBattleCamera
    (:Success
      ;;[0 0 0] Addes Battle UI
      (bind _returnvalue (UserInterface|CreateWidget "/Game/Blueprints/UI/BattleUI_BP.BattleUI_BP_C" 0 (Variables|Default|GetCurrentBattle)))
      (bind _output_get (Variables|Default|SetBattleUI _returnvalue))
      (UserInterface|Viewport|AddtoViewport _output_get 0)
      (Variables|/Game/Blueprints/UI/BattleUI_BP.BattleUI_BP_C|SetInBattle? _output_get true)
      ;[1 0 0] Testing Battle Over and Switching to Playable Tidus
      (Utilities|FlowControl|Delay 5.0)
      (CallFunction|BattleOver))))

(event Custom|Battle%20Over
  (bind _battleui (Variables|Default|GetBattleUI))
  ;[0 0 0] Battle Over
  (CallFunction|SwitchtoExploreMode)
  ;;[0 0 0] Hides/Disables Battle UI
  (Widget|SetVisibility _battleui "Collapsed")
  (Variables|/Game/Blueprints/UI/BattleUI_BP.BattleUI_BP_C|SetInBattle? _battleui false)
  (Default|RemoveUnits (Variables|Default|GetCurrentBattle)))

(event Custom|SwitchToExploreMode
  (bind _ffxgamemode (Variables|Default|GetFFXGameMode))
  ;[0 0 0] Switches Back to Explore Mode and Playable Tidus
  (Variables|/Game/Blueprints/FFXGameMode_BP.FFXGameMode_BP_C|SetCurrentGameState _ffxgamemode "NewEnumerator0")
  (Default|EnablePlayerInput _ffxgamemode)
  (Utilities|SwitchtoPlayerCamera
    (:Success
      (Variables|/Game/Blueprints/FFXGameMode_BP.FFXGameMode_BP_C|SetInBattle? _ffxgamemode false))))

(fn ConstructionScript)