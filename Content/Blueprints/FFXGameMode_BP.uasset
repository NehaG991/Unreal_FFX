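; Game mode for a Final Fantasy X-style RPG that holds shared party, exploration and battle state.
; BeginPlay adds Tidus to the party, caches the player character and controller, and takes the first actor on the TestBattleSpace layer as the current battle space.
; Its events toggle move input and mesh animation pausing, start battles through that space, and randomize the encounter timer.
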(event Custom|Randomize%20Encounter%20Timer
  ;[0 0 0] Randomizes Encounter Timer
  (Variables|Default|SetRandomEncounterTimer (Math|Random|RandomFloatinRange 1e+01 2e+01)))

(event Custom|StartBattle
  ;[0 0 0] Starts Battles
  (Variables|Default|SetInBattle? true)
  (Default|InitBattle (Variables|Default|GetCurrentBattleSpace)))

(event Custom|Disable%20Player%20Input
  ;[0 0 0] Disable/Enable Player Input & Pauses Animations
  (Input|SetIgnoreMoveInput (Variables|Default|GetFFXPlayerController) true)
  (Variables|/Script/Engine.SkeletalMeshComponent|SetbPauseAnims (Variables|/Script/Engine.Character|GetMesh (Variables|Default|GetPlayableTidus)) true))

(event Custom|Enable%20Player%20Input
  ;[0 0 0] Disable/Enable Player Input & Pauses Animations
  (Input|SetIgnoreMoveInput (Variables|Default|GetFFXPlayerController) false)
  (Variables|/Script/Engine.SkeletalMeshComponent|SetbPauseAnims (Variables|/Script/Engine.Character|GetMesh (Variables|Default|GetPlayableTidus)) false))

(event EventBeginPlay
  ;[0 0 0] Adding Tidus to Party
  (bind _astidus_bp (Utilities|Casting|CastToTidus_BP (Game|GetPlayerCharacter 0)))
  (Variables|Default|SetPlayableTidus _astidus_bp)
  (Utilities|Array|SetArrayElem (Variables|Default|GetParty) 0 "Tidus")
  ;[0 0 0] Saves Player Controller as Variable
  (bind _asffxplayer_controller_bp (Utilities|Casting|CastToFFXPlayerController_BP (Game|GetPlayerController 0)))
  (Variables|Default|SetFFXPlayerController _asffxplayer_controller_bp)
  ;[0 0 0] Adds Test Battle Actor Reference
  (bind _returnvalue (Class|LayersBlueprintLibrary|GetActors (Utilities|Struct|MakeActorLayer "TestBattleSpace")))
  (bind _asbattle_base_bp (Utilities|Casting|CastToBattleBase_BP (Utilities|Array|Get(acopy) _returnvalue)))
  (Variables|Default|SetCurrentBattleSpace _asbattle_base_bp))

(fn ConstructionScript)